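; Player controller for DohMansLand that binds keyboard shortcuts for quitting, testing and display setup.
; T quits the game, while B and N are test keys that give every BP_BaseTank a bouncy bullets or juggernaut powerup component.
; F builds a fullscreen resolution console command from the desktop resolution, then sets screen percentage and disables global illumination.
; An unconnected touch hit-test debug print never runs.
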(event Input|KeyboardEvents|F
  (params (Key :type Key%20Structure :default "None"))
  (:Released
    (bind _returnvalue (Settings|GetGameUserSettings))
    (Development|ExecuteConsoleCommand (Utilities|String|Append "r.setres " (Utilities|String|ToString(Integer) (.x (Class|GameUserSettings|GetDesktopResolution _returnvalue))) "x" (Utilities|String|ToString(Integer) (.y (Class|GameUserSettings|GetDesktopResolution _returnvalue))) " f") 0)
    (Development|ExecuteConsoleCommand "r.ScreenPercentage 100" 0)
    (Development|ExecuteConsoleCommand "showflag.globalillumination 0" 0)))

(event Input|KeyboardEvents|T
  (params (Key :type Key%20Structure :default "None"))
  (:Pressed
    (Game|QuitGame 0 "Quit" false)))

(event Input|KeyboardEvents|N
  (params (Key :type Key%20Structure :default "None"))
  ;[1 1 1] for testing purposes
  (:Pressed
    (bind _outactors (Actor|GetAllActorsOfClass "/Game/Blueprints/Player/BP_BaseTank.BP_BaseTank_C"))
    (for _array_element _outactors
      (Game|AddComponentbyClass _array_element "/Game/Blueprints/PowerupComponents/Movement/AC_JuggernautPowerup.AC_JuggernautPowerup_C"))))

(event Input|KeyboardEvents|B
  (params (Key :type Key%20Structure :default "None"))
  ;[1 1 1] for testing purposes
  (:Pressed
    (bind _outactors (Actor|GetAllActorsOfClass "/Game/Blueprints/Player/BP_BaseTank.BP_BaseTank_C"))
    (for _array_element _outactors
      (Game|AddComponentbyClass _array_element "/Game/Blueprints/PowerupComponents/Weapons/AC_BouncyBulletsPowerup.AC_BouncyBulletsPowerup_C"))))

(event Input|TouchEvents|InputTouch
  (params (Location :type Vector) (FingerIndex :type ETouchIndex%20Enum)))

(fn ConstructionScript)