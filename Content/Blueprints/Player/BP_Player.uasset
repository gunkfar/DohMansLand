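; Per-player touch control panel for DohMansLand that spawns and drives that player's tank.
; Touching join slides in 3D controls tinted with GameMode tank colors and spawns the tank.
; Tick converts tracked fingers on twin joysticks and an aim gear into differential steering and turret rotation, while a button fires.
; Death retracts controls and runs a dial timer scaled by death count before respawning; the first death also removes unjoined players.
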(event OnInputTouchBegin(JoinInteract)
  (params (FingerIndex :type ETouchIndex%20Enum :default "Touch1") (TouchedComponent :type Primitive%20Component%20Object%20Reference))
  ;[1 0.5 0.5] NotPlaying --> Playing
  ;;[0.2 0.2 0.2] Removes the join button and moves the controls forward
  (Audio|PlaySound2D "/Game/Assets/SFX/misc_outside_noises/Xylo/SFXQ_Xylo.SFXQ_Xylo" 1.0 1.0 0.0 0 0)
  (Components|DestroyComponent (Variables|Default|GetJoinInteract))
  (Variables|Gameplay|SetEPlayerState "NewEnumerator1")
  (Default|CallGameStart (CallFunction|GetDohMansLandGameMode))
  (Utilities|FlowControl|Sequence
    (:then_0
      (Utilities|MoveComponentto0 (Variables|Default|GetControllerBase) 1.0))
    (:then_1
      (Utilities|MoveComponentto0 (Variables|Default|GetGears) 1.2))
    (:then_2
      (Variables|TouchBooleans|SetbIsReceivingInput true)
      (CallFunction|SpawnTank))))

(event OnInputTouchBegin(SpinnerCollision)
  (params (FingerIndex :type ETouchIndex%20Enum :default "Touch1") (TouchedComponent :type Primitive%20Component%20Object%20Reference))
  ;[1 0.5 1] Sets touch indicies when a component is touched
  (if (Variables|TouchBooleans|GetbIsReceivingInput)
    (if (not (Variables|TouchBooleans|GetbRotateTurret))
      (Variables|TouchBooleans|SetbRotateTurret true)
      (Variables|TouchIndicies|SetTurretIndex FingerIndex))))

(event OnInputTouchBegin(FireCollision)
  (params (FingerIndex :type ETouchIndex%20Enum :default "Touch1") (TouchedComponent :type Primitive%20Component%20Object%20Reference))
  ;[1 1 0.5] FIRE BUTTON LOGIC
  ;;[0.2 0.2 0.2] Fires projectile when button is pressed
  (if (not (Variables|TouchBooleans|GetbFireButton))
    (Variables|TouchBooleans|SetbFireButton true)
    (CallFunction|MoveButton 0.01 "0, 0,-800.000000")
    (Default|FireProjectile (Variables|Default|GetTankRef))))

(event OnInputTouchBegin(LeftInteraction)
  (params (FingerIndex :type ETouchIndex%20Enum :default "Touch1") (TouchedComponent :type Primitive%20Component%20Object%20Reference))
  ;[1 0.5 1] Sets touch indicies when a component is touched
  (if (Variables|TouchBooleans|GetbIsReceivingInput)
    (if (not (Variables|TouchBooleans|GetbRotateLeftStick))
      (Variables|TouchBooleans|SetbRotateLeftStick true)
      (Variables|TouchIndicies|SetLeftMoveIndex FingerIndex))))

(event OnInputTouchBegin(RightInteraction)
  (params (FingerIndex :type ETouchIndex%20Enum :default "Touch1") (TouchedComponent :type Primitive%20Component%20Object%20Reference))
  ;[1 0.5 1] Sets touch indicies when a component is touched
  (if (Variables|TouchBooleans|GetbIsReceivingInput)
    (if (not (Variables|TouchBooleans|GetbRotateRightStick))
      (Variables|TouchBooleans|SetbRotateRightStick true)
      (Variables|TouchIndicies|SetRightMoveIndex FingerIndex))))

(event OnInputTouchEnd(FireCollision)
  (params (FingerIndex :type ETouchIndex%20Enum :default "Touch1") (TouchedComponent :type Primitive%20Component%20Object%20Reference))
  ;[1 1 0.5] FIRE BUTTON LOGIC
  ;;[0.2 0.2 0.2] Moves the button up when released
  (if (Variables|TouchBooleans|GetbFireButton)
    (Variables|TouchBooleans|SetbFireButton false)
    (CallFunction|MoveButton 0.05 "0, 0,-400.000000")))

(event Custom|Move%20Button
  (params (Over%20Time :type Float%20%28double-precision%29) (Location :type Vector))
  (bind _firebutton (Variables|Default|GetFireButton))
  ;[1 1 0.5] FIRE BUTTON LOGIC
  ;;[0.2 0.2 0.2] Function for moving the button up and down when pressed/released
  (Components|MoveComponentTo _firebutton Location (Variables|/Script/Engine.SceneComponent|GetRelativeRotation _firebutton) false false Over%20Time false))

(event Custom|TankDeath
  (params (Hit :type Hit%20Result%20Structure))
  (bind _tankref (Variables|Default|GetTankRef))
  (bind _tankref_2 (Variables|Default|GetTankRef))
  ;[0.5 0.5 1] Tank Death
  ;;[0.2 0.2 0.2] Disables and removes controls, while spawning the explosion, setting the player state enum to Dead, and checking for a win
  (Utilities|FlowControl|Sequence
    (:then_0
      (Default|CallTankDeath (CallFunction|GetDohMansLandGameMode) _tankref)
      (Audio|Components|Audio|Stop (Variables|/Game/Blueprints/Player/BP_BaseTank.BP_BaseTank_C|GetMoveSound _tankref))
      (Variables|TouchBooleans|SetbIsReceivingInput false)
      (bind _result (Math|Integer|IncrementInt (Variables|Respawn|GetNumberOfDeaths))
        (:%20%20
          (Variables|Respawn|SetRespawnTime (* _result (Variables|Respawn|GetBaseRespawnTime)))
          (Rendering|Material|SetVectorParameterValue (Variables|Materials|GetControllerDynamicMaterials) "Color" "(R=0.200000,G=0.200000,B=0.200000,A=1.000000)" :!class /Script/Engine.MaterialInstanceDynamic)
          (Utilities|RemoveControls))))
    (:then_1
      (if (Variables|Respawn|GetbDeathByTimeout)
        (Actor|DestroyActor (Variables|Default|GetTankRef))
        (else
          (bind _returnvalue (Niagara|SpawnSystematLocation "/Game/Assets/FX/Explosions/FX_TankExplosion.FX_TankExplosion" (Transformation|GetActorLocation (Variables|Default|GetTankRef))))
          (Class|NiagaraComponent|SetVariableStaticMesh _returnvalue "user.tankMesh" (Variables|/Script/Engine.StaticMeshComponent|GetStaticMesh (Variables|/Game/Blueprints/Player/BP_BaseTank.BP_BaseTank_C|GetTankBase _tankref_2)))
          (Utilities|FlowControl|Sequence
            (:then_0
              (if (Variables|Gameplay|GetbRemovedControls)
                _
                (else
                  (bind _outactors (Actor|GetAllActorsOfClass "BP_Player_C"))
                  (for _array_element _outactors
                    (Default|CallRemoveInactivePlayers _array_element))))
              (Variables|Gameplay|SetEPlayerState "NewEnumerator2")
              (CallFunction|StartRespawnTimer)
              (Default|CheckforWin (CallFunction|GetDohMansLandGameMode)))
            (:then_1
              (Utilities|FlowControl|Delay 3.0)
              (Actor|DestroyActor _tankref_2))))))))

(event Custom|TickTimer
  (bind _respawntimerdial (Variables|Default|GetRespawnTimerDial))
  ;[0.5 1 0.5] Respawn Timer
  (Transformation|AddRelativeRotation _respawntimerdial (Math|Rotator|MakeRotator 0.0 0.0 -6.0) false false)
  (if (Math|Float|NearlyEqual(Float) (.yaw (Variables|/Script/Engine.SceneComponent|GetRelativeRotation _respawntimerdial)) 0.0 3.0)
    (CallFunction|ClearandRemoveTimer)
    (Variables|TouchBooleans|SetbIsReceivingInput true)
    (Utilities|FlowControl|Sequence
      (:then_0
        (Utilities|MoveComponentto0 (Variables|Default|GetControllerBase) 1.0))
      (:then_1
        (Utilities|MoveComponentto0 (Variables|Default|GetGears) 1.2))
      (:then_2
        (Variables|TouchBooleans|SetbIsReceivingInput true)
        (CallFunction|SpawnTank))
      (:then_3
        (CallFunction|SetAllMaterials)
        (Variables|Gameplay|SetEPlayerState "NewEnumerator1")))))

(event Custom|StartRespawnTimer
  ;[0.5 1 0.5] Respawn Timer
  (Utilities|MoveComponentto0 (Variables|Default|GetRespawnTimerBase) 1.0
    (:Completed
      (bind _returnvalue (Utilities|Time|SetTimerbyEvent (EventDispatchers|CreateEvent :!event Custom|TickTimer) (/ (Variables|Respawn|GetRespawnTime) 6e+01) true))
      (Variables|Respawn|SetRespawnTimerHandle _returnvalue))))

(event Custom|RemoveInactiveControls
  ;[0.5 0.5 1] Tank Death
  ;;[0.2 0.2 0.2] After the first tank death, removes all players that are not playing
  (Variables|Gameplay|SetbRemovedControls true)
  (switch Utilities|FlowControl|Switch|SwitchonEPlayerState (Variables|Gameplay|GetEPlayerState)
    (:NewEnumerator0
      (Variables|Respawn|SetbDeathByTimeout true)
      (Utilities|RemoveControls)
      (Actor|DestroyActor))))

(event Custom|ClearAndRemoveTimer
  (bind _respawntimerbase (Variables|Default|GetRespawnTimerBase))
  (bind _relativelocation (Variables|/Script/Engine.SceneComponent|GetRelativeLocation _respawntimerbase))
  ;[0.5 1 0.5] Respawn Timer
  (Utilities|Time|ClearandInvalidateTimerbyHandle (Variables|Respawn|GetRespawnTimerHandle))
  (Components|MoveComponentTo _respawntimerbase (Math|Vector|MakeVector -7e+03 (.y _relativelocation) (.z _relativelocation)) (Variables|/Script/Engine.SceneComponent|GetRelativeRotation _respawntimerbase) true true 1.0 false))

(event EventBeginPlay
  (bind _xylophonematerial (Variables|Default|GetXylophoneMaterial))
  ;[1 1 1] Initialization has to be done here because we need the GM to build first for colors
  ;;[0.2 0.2 0.2] Set material colors and bind events
  (Variables|Default|SetTankVariables (Utilities|Array|Get(acopy) (Variables|/Game/Blueprints/Player/BP_DohMansLand_GameMode.BP_DohMansLand_GameMode_C|GetTank%20Variables (CallFunction|GetDohMansLandGameMode)) (Variables|Gameplay|GetPlayerIndex)))
  (EventDispatchers|BindEventtoRemoveInactivePlayers (EventDispatchers|CreateEvent :!event Custom|RemoveInactiveControls))
  (CallFunction|SetAllMaterials)
  (if (== (Variables|Gameplay|GetPlayerIndex) (Variables|/Game/Blueprints/Player/BP_DohMansLand_GameInstance.BP_DohMansLand_GameInstance_C|GetWinnerID (CallFunction|GetDohMansLandGameInstance)))
    (Rendering|Material|SetScalarParameterValue _xylophonematerial "HasWon" 1.0 :!class /Script/Engine.MaterialInstanceDynamic)
    (else
      (Rendering|Material|SetScalarParameterValue _xylophonematerial "HasWon" 0.0 :!class /Script/Engine.MaterialInstanceDynamic))))

(event EventTick
  (params (DeltaSeconds :type Float%20%28single-precision%29))
  (bind (_rotationaxis _forwardaxis) (CallFunction|GetAxisValuesfromJoysticks))
  (bind _tankref (Variables|Default|GetTankRef))
  ;[0.5 1 1] Add control inputs to components
  (if (Variables|TouchBooleans|GetbIsReceivingInput)
    (Utilities|FlowControl|Sequence
      (:then_0
        (|SetSpinnerRotation))
      (:then_1
        (|SetLeftStickRotation))
      (:then_2
        (|SetRightStickRotation))
      (:then_3
        (Default|RotateBody _tankref _rotationaxis))
      (:then_4
        (Default|MoveTank _tankref _forwardaxis))
      (:then_5
        (Default|RotateTurret _tankref (.yaw (Transformation|GetWorldRotation (Variables|Default|GetSpinner))) (Variables|TouchBooleans|GetbResetTurretZ))))
    (else
      (CallFunction|ResetJoysticks))))

(fn ConstructionScript)

(fn SetAllMaterials
  (|SetRespawnTimerColors)
  (|SetControllerColors))

(fn GetAxisValuesfromJoysticks
  (bind _joystickexponent (Variables|Movement|GetJoystickExponent))
  (bind _rightswitch (Variables|Default|GetRightSwitch))
  (bind _leftswitch (Variables|Default|GetLeftSwitch))
  (bind _relativerotation (Variables|/Script/Engine.SceneComponent|GetRelativeRotation _rightswitch))
  (bind _relativerotation_2 (Variables|/Script/Engine.SceneComponent|GetRelativeRotation _leftswitch))
  (bind _returnvalue (/ (.roll _relativerotation) 45.0))
  (bind _returnvalue_2 (/ (.roll _relativerotation_2) 45.0))
  (bind _returnvalue_3 (Utilities|FindControlPower _returnvalue_2 _joystickexponent))
  (bind _returnvalue_4 (Utilities|FindControlPower _returnvalue _joystickexponent))
  (bind _returnvalue_5 (/ _returnvalue_3 2.0))
  (bind _returnvalue_6 (/ _returnvalue_4 2.0))
  (return (* (+ (* _returnvalue_6 -1.0) _returnvalue_5) (Variables|Movement|GetTurnSpeed)) (+ _returnvalue_6 _returnvalue_5)))

(fn SpawnTank
  (bind _returnvalue (Game|SpawnActorfromClass "/Game/Blueprints/Player/BP_BaseTank.BP_BaseTank_C" (Transformation|GetWorldTransform (Variables|Default|GetSpawnPoint)) "AdjustIfPossibleButAlwaysSpawn" 0 (Variables|Default|GetTankVariables) self (Variables|Gameplay|GetPlayerIndex) 0))
  (Variables|Default|SetTankRef _returnvalue)
  (bind _returnvalue_2 (Game|SpawnActorfromClass "/Game/Blueprints/Player/BP_DohMansLand_PlayerController.BP_DohMansLand_PlayerController_C" (Math|Transform|MakeTransform "0, 0, 0" "0, 0, 0" "1.000000,1.000000,1.000000") "Undefined" 0 0))
  (Pawn|Possess _returnvalue_2 (Variables|Default|GetTankRef)))

(fn ResetJoysticks
  (Transformation|SetRelativeRotation (Variables|Default|GetLeftSwitch) "0, 0, 0" false false)
  (Transformation|SetRelativeRotation (Variables|Default|GetRightSwitch) "0, 0, 0" false false))