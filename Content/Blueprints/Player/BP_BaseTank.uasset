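; Base player tank pawn that handles movement, turret aiming, shooting, powerup components, lives and the winner's celebration.
; Construction applies per-player meshes from the game mode, socket-attaches turret parts and registers the scene capture with spectator screens.
; Firing is rate-gated and capped by active projectiles, with a delayed clear allowing extra shots.
; Lives drive Juggernaut effects and death, while winners get a crown, alternate camera and confetti shots.
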(event Custom|RotateTurret
  (params (TargetRotation :type Float%20%28double-precision%29) (bResetZ :type Boolean))
  (bind _collision (Variables|Default|GetCollision))
  (bind _turret (Variables|Default|GetTurret))
  (bind _returnvalue (Transformation|GetRelativeTransform _collision))
  (bind _relativerotation (Variables|/Script/Engine.SceneComponent|GetRelativeRotation _turret))
  (bind _returnvalue_2 (Math|Transform|InverseTransformRotation _returnvalue (Math|Rotator|MakeRotator 0.0 0.0 TargetRotation)))
  (bind _returnvalue_3 (select bResetZ 0.0 (.yaw _returnvalue_2)))
  ;[0.3 1 1] MOVEMENT AND ROTATION
  ;;[0.2 0.2 0.2] Rotate the turret based on the spinner input
  (Components|MoveComponentTo _turret (Variables|/Script/Engine.SceneComponent|GetRelativeLocation _turret) (Math|Rotator|MakeRotator (.roll _relativerotation) (.pitch _relativerotation) _returnvalue_3) false false (Utilities|GetDistanceConvertedtoTime _returnvalue_3 (.yaw _relativerotation)) false))

(event Custom|RotateBody
  (params (AxisValue :type Float%20%28double-precision%29))
  ;[0.3 1 1] MOVEMENT AND ROTATION
  ;;[0.2 0.2 0.2] Rotate the body
  (Variables|Treads|SetTreadSpeed (Math|Vector2D|MakeVector2D (.x (Variables|Treads|GetTreadSpeed)) 0.0))
  (Class|Actor|AddActorWorldRotation (Math|Rotator|MakeRotator 0.0 0.0 (* AxisValue (Variables|Movement|GetMoveSpeed) (Variables|Movement|GetDeltaSeconds) -1.0))))

(event Custom|MoveTank
  (params (AxisValue :type Float%20%28double-precision%29))
  ;[0.3 1 1] MOVEMENT AND ROTATION
  ;;[0.2 0.2 0.2] Moves the tank forward
  (Variables|Treads|SetTreadSpeed (Math|Vector2D|MakeVector2D AxisValue (.y (Variables|Treads|GetTreadSpeed))))
  (Class|PawnMovementComponent|AddInputVector (Variables|Default|GetFloatingPawnMovement) (* AxisValue (Variables|Movement|GetMoveSpeed) (Variables|Movement|GetDeltaSeconds) (Transformation|GetActorForwardVector) -1.0) false)
  (if (Math|Float|NearlyEqual(Float) AxisValue 0.0 1e-06)
    (Utilities|IsValid (Variables|Default|GetMoveSound)
      (:Is%20Valid
        (Audio|Components|Audio|Stop (Variables|Default|GetMoveSound))
        (goto _label Reset)))
    (else
      (Utilities|FlowControl|DoOnce false :!label _label
        (:Completed
          (bind _returnvalue (Audio|SpawnSoundatLocation (.movesound (Variables|Gameplay|GetTankVariables)) (Transformation|GetActorLocation) "0, 0, 0" 1.0 1.0 0.0 0 0))
          (Variables|Default|SetMoveSound _returnvalue))))))

(event Custom|FireProjectile
  (bind _barrel (Variables|Default|GetBarrel))
  ;[1 0.3 1] SHOOTING
  ;;[0.2 0.2 0.2] Shoots a projectile
  (if (not (>= (Utilities|Array|Length (Variables|Projectiles|GetActiveProjectiles)) (Variables|Projectiles|GetMaxProjectiles)))
    (Utilities|FlowControl|Sequence
      (:then_0
        (Utilities|FlowControl|DoOnce false :!label _label
          (:Completed
            (Utilities|SpawnTurretParticles)
            (if (Variables|Gameplay|GetbHasWon)
              (Audio|PlaySound2D "/Game/Assets/SFX/misc_outside_noises/Victory_sounds/SFXQ_Tank_Party_Horn.SFXQ_Tank_Party_Horn" 1.0 1.0 0.0 0 0)
              (else
                (bind _returnvalue (Game|SpawnActorfromClass (Variables|Projectiles|GetProjectileClass) (Math|Transform|MakeTransform (Transformation|GetWorldLocation _barrel) (Transformation|GetWorldRotation _barrel) "1.000000,1.000000,1.000000") "Undefined" 0 self 0))
                (Utilities|Array|Add (Variables|Projectiles|GetActiveProjectiles) _returnvalue)
                (Audio|PlaySoundatLocation (Variables|/Game/Blueprints/Projectiles/BP_BaseProjectile.BP_BaseProjectile_C|GetShoot%20Sound _returnvalue) (Transformation|GetActorLocation) "0, 0, 0" 1.0 1.0 0.0 0 0 0 0)))
            (Utilities|FlowControl|Delay (Variables|/Game/Blueprints/Projectiles/BP_BaseProjectile.BP_BaseProjectile_C|GetFireRate _returnvalue))
            (goto _label Reset))))
      (:then_1
        (Utilities|FlowControl|Delay 2.0)
        (Utilities|Array|Clear (Variables|Projectiles|GetActiveProjectiles)) ; this just makes shooting\nmore fun, allows for more than 3 projs without\nhaving to wait for a despawn
      ))))

(event Custom|AddPowerup
  (params (Powerup :type AC%20Base%20Powerup%20Class%20Reference))
  ;[0.2 0.2 0.2] Adds the powerup to the tank
  (Game|AddComponentbyClass Powerup))

(event Custom|SetWinner
  (bind _particlevalues (Variables|Default|GetParticleValues))
  ;[0.2 0.2 0.2] Sets variables for when a player wins
  (Utilities|FlowControl|Sequence
    (:then_0
      (Variables|Gameplay|SetbHasWon true)
      (Rendering|SetVisibility (Variables|Default|GetCrown) true false)
      (Transformation|AttachComponentToComponent (Variables|Default|GetSceneCaptureComponent2D) (Variables|Default|GetTurret) "WinCamera" "KeepRelative" "KeepRelative" "KeepRelative" true))
    (:then_1
      (Variables|/Game/Assets/FX/BP_NiagaraValueHolder.BP_NiagaraValueHolder_C|SetSystem _particlevalues "/Game/Assets/FX/Bullet/FX_Confetti.FX_Confetti")
      (Transformation|SetRelativeScale3D _particlevalues "4.000000,4.000000,4.000000")
      (Variables|/Game/Assets/FX/BP_NiagaraValueHolder.BP_NiagaraValueHolder_C|SetColor%20Param _particlevalues (.tankcolor (Variables|Gameplay|GetTankVariables))))))

(event Custom|RemoveProjectile
  (params (Projectile :type BP%20Base%20Projectile%20Object%20Reference))
  ;[1 0.3 1] SHOOTING
  ;;[0.2 0.2 0.2] Removes projectiles when they die
  (Utilities|Array|RemoveItem (Variables|Projectiles|GetActiveProjectiles) Projectile))

(event EventTick
  (params (DeltaSeconds :type Float%20%28single-precision%29))
  (bind _treadspeed (Variables|Treads|GetTreadSpeed))
  ;[0.2 0.2 0.2] Updates the treads based on the speed of the tank
  (Variables|Movement|SetDeltaSeconds DeltaSeconds)
  (if (Utilities|Operators|EqualEqual (Variables|Treads|GetTreadSpeed) (Variables|Treads|GetPreviousTreads) 0.01)
    _
    (else
      (Default|UpdateSpeeds (Variables|Default|GetTreads) (.y _treadspeed) (.x _treadspeed))
      (Variables|Treads|SetPreviousTreads (Variables|Treads|GetTreadSpeed))))
  (Effects|Components|ParticleSystem|SetFloatParameter (Variables|Default|GetExhaust) "user.tankSpeed" (Math|Vector|VectorLength (Transformation|GetVelocity))))

(event EventBeginPlay
  ;[0.2 0.2 0.2] Attaches the camera to a differnt scoket if the tank won the last round
  (EventDispatchers|BindEventtoGameOver (CallFunction|GetDohMansLandGameMode) (EventDispatchers|CreateEvent :!event Custom|SetWinner))
  (if (== (Variables|/Game/Blueprints/Player/BP_DohMansLand_GameInstance.BP_DohMansLand_GameInstance_C|GetWinnerID (CallFunction|GetDohMansLandGameInstance)) (Variables|Gameplay|GetPlayerIndex))
    (Rendering|SetVisibility (Variables|Default|GetCrown) true false)
    (Transformation|AttachComponentToComponent (Variables|Default|GetSceneCaptureComponent2D) (Variables|Default|GetTurret) "WinCamera" "KeepRelative" "KeepRelative" "KeepRelative" true)))

(fn ConstructionScript
  (bind _returnvalue (CallFunction|GetDohMansLandGameMode))
  (bind _playerindex (Variables|Gameplay|GetPlayerIndex))
  (bind _tank_variables (Variables|/Game/Blueprints/Player/BP_DohMansLand_GameMode.BP_DohMansLand_GameMode_C|GetTank%20Variables _returnvalue))
  (bind _output (Utilities|Array|Get(acopy) _tank_variables _playerindex))
  (Utilities|FlowControl|Sequence
    (:then_0
      (Utilities|FlowControl|Sequence
        (:then_0
          (Components|StaticMesh|SetStaticMesh (Variables|Default|GetTankBase) (.basemesh _output))
          (Components|StaticMesh|SetStaticMesh (Variables|Default|GetTurret) (.turretmesh _output))
          (Variables|Gameplay|SetDefaultTurretMesh (.turretmesh _output)))))
    (:then_1
      (Transformation|AttachComponentToComponent (Variables|Default|GetSceneCaptureComponent2D) (Variables|Default|GetTurret) "Camera" "KeepRelative" "KeepRelative" "KeepRelative" true)
      (Transformation|AttachComponentToComponent (Variables|Default|GetBarrel) (Variables|Default|GetTurret) "Barrel" "KeepRelative" "KeepRelative" "KeepRelative" true)
      (Transformation|AttachComponentToComponent (Variables|Default|GetParticleValues) (Variables|Default|GetTurret) "Barrel" "KeepRelative" "KeepRelative" "KeepRelative" true)
      (Transformation|AttachComponentToComponent (Variables|Default|GetCrown) (Variables|Default|GetTurret) "Crown" "KeepRelative" "KeepRelative" "KeepRelative" true)
      (bind _outactors (Actor|GetAllActorsOfClass "/Game/Blueprints/MapItems/BP_SpectatorScreen.BP_SpectatorScreen_C"))
      (for _array_element _outactors
        (Utilities|Map|Add (Variables|/Game/Blueprints/MapItems/BP_SpectatorScreen.BP_SpectatorScreen_C|GetRenderTargets _array_element) (Variables|Gameplay|GetPlayerIndex) (Variables|Default|GetSceneCaptureComponent2D))))))

(fn SetJuggernautLives
  (bind _controllerreference (Variables|Gameplay|GetControllerReference))
  (bind _lives (Variables|/Game/Blueprints/Player/BP_Player.BP_Player_C|GetLives _controllerreference))
  (bind _returnvalue (- _lives 1))
  ;[0.2 0.2 0.2] Adds the visuals for jug
  (if (> _returnvalue 0)
    (Utilities|FlowControl|Sequence
      (:then_0
        (if (Utilities|IsValid (Variables|Gameplay|GetJugParts))
          (Components|DestroyComponent (Variables|Gameplay|GetJugParts))))
      (:then_1
        (bind _returnvalue_2 (Niagara|SpawnSystemAttached "/Game/Assets/FX/Tank/FX_JugActive_System.FX_JugActive_System" (Variables|Default|GetTankBase) "None" "0, 0, 0" "0, 0, 0" "SnapToTargetIncludingScale" true))
        (bind _output_get (Variables|Gameplay|SetJugParts _returnvalue_2))
        (Class|NiagaraComponent|SetVariableInt _output_get "lives" _returnvalue)))
    (elif (Utilities|IsValid (Variables|Gameplay|GetJugParts))
      (Components|DestroyComponent (Variables|Gameplay|GetJugParts))
      (Variables|Gameplay|SetJugParts 0))))

(fn DecrementLives
  (params (Projectile :type BP%20Base%20Projectile%20Object%20Reference) (Hit :type Hit%20Result%20Structure))
  (bind _controllerreference (Variables|Gameplay|GetControllerReference))
  (Utilities|Casting|CastToBP_BigProjectile Projectile
    (:then
      (Variables|/Game/Blueprints/Player/BP_Player.BP_Player_C|SetLives _controllerreference (- (Variables|/Game/Blueprints/Player/BP_Player.BP_Player_C|GetLives _controllerreference) (* (Math|Integer|Clamp(Integer) (Utilities|Array|Length (Actor|GetComponentsByClass "/Game/Blueprints/PowerupComponents/Weapons/AC_BigProjectilesPowerup.AC_BigProjectilesPowerup_C")) 0 2) 3))))
    (:CastFailed
      (bind _result (Math|Integer|DecrementInt (Variables|/Game/Blueprints/Player/BP_Player.BP_Player_C|GetLives (Variables|Gameplay|GetControllerReference)))
        (:%20%20
          _))))
  (CallFunction|SetJuggernautLives)
  (if (<= _result 0)
    (Default|TankDeath (Variables|Gameplay|GetControllerReference) Hit)
    (Audio|PlaySoundatLocation (.explosionsound (Variables|Gameplay|GetTankVariables)) (Transformation|GetActorLocation) "0, 0, 0" 1.0 1.0 0.0 0 0 0 0)
    (Camera|PlayWorldCameraShake "/Game/Blueprints/MapItems/Bp_CameraShake.Bp_CameraShake_C" (Camera|GetCameraLocation (Game|GetPlayerCameraManager 0)) 0.0 5e+08)
    (for _array_element (Actor|GetComponentsByClass "/Game/Blueprints/PowerupComponents/AC_BasePowerup.AC_BasePowerup_C")
      (Components|DestroyComponent _array_element))))

(fn AddSpeedVisuals
  (Utilities|FlowControl|Sequence
    (:then_0
      (bind _returnvalue (AddComponent|AddStaticMeshComponent true))
      (Transformation|AttachComponentToComponent _returnvalue (Variables|Default|GetTankBase) "RightEngine" "KeepRelative" "KeepRelative" "SnapToTarget" true)
      (Niagara|SpawnSystemAttached "/Game/Assets/FX/Tank/FX_BubbleExhaust.FX_BubbleExhaust" _returnvalue "EngineParticle" "0, 0, 0" "0, 0, 0" "KeepRelativeOffset" false))
    (:then_1
      (bind _returnvalue_2 (AddComponent|AddStaticMeshComponent true))
      (Transformation|AttachComponentToComponent _returnvalue_2 (Variables|Default|GetTankBase) "LeftEngine" "KeepRelative" "KeepRelative" "SnapToTarget" true)
      (bind _returnvalue_3 (Niagara|SpawnSystemAttached "/Game/Assets/FX/Tank/FX_BubbleExhaust.FX_BubbleExhaust" _returnvalue_2 "EngineParticle" "0, 0, 0" "0, 0, 0" "KeepRelativeOffset" false))
      (Transformation|SetWorldScale3D _returnvalue_3 "1.000000,1.000000,1.000000"))))