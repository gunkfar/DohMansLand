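; BP_BaseWall is a base wall Blueprint that registers itself as a spawnable asset for procedural generation.
; On BeginPlay it enables mesh physics and, if PlacedInLevel is set, finds every BP_AssetGenerator.
; It adds its class, spawn cap and frequency to each generator's Large, Medium or Small asset list according to SizeEnum.
; A PlayHitSound function plays the hit sound at the wall's location.
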(event EventBeginPlay
  (bind _self self)
  (bind _maxnumberofasset (Variables|Spawning|GetMaxNumberOfAsset))
  (bind _frequency (Variables|Spawning|GetFrequency))
  (bind _returnvalue (Utilities|GetClass _self))
  (bind _fassetspawninginfo (Utilities|Struct|MakeFAssetSpawningInfo _returnvalue _maxnumberofasset _frequency))
  ;[1 1 1] set info for spawning on BP_AssetGenerator
  (Physics|SetSimulatePhysics (Variables|Default|GetMesh) true)
  (if (Variables|Default|GetbPlacedInLevel)
    (bind _outactors (Actor|GetAllActorsOfClass "/Game/Blueprints/Generation/BP_AssetGenerator.BP_AssetGenerator_C"))
    (for _array_element _outactors
      (switch Utilities|FlowControl|Switch|SwitchonEAssetSizeEnum (Variables|Default|GetSizeEnum)
        (:NewEnumerator0
          (Utilities|Array|Add (Variables|/Game/Blueprints/Generation/BP_AssetGenerator.BP_AssetGenerator_C|GetLargeAssets _array_element) _fassetspawninginfo))
        (:NewEnumerator1
          (Utilities|Array|Add (Variables|/Game/Blueprints/Generation/BP_AssetGenerator.BP_AssetGenerator_C|GetMediumAssets _array_element) _fassetspawninginfo))
        (:NewEnumerator2
          (Utilities|Array|Add (Variables|/Game/Blueprints/Generation/BP_AssetGenerator.BP_AssetGenerator_C|GetSmallAssets _array_element) _fassetspawninginfo))))))

(fn ConstructionScript)

(fn PlayHitSound
  (Audio|PlaySoundatLocation (Variables|Sound|GetHitSound) (Transformation|GetActorLocation) "0, 0, 0" 1.0 1.0 0.0 0 0 0 0))