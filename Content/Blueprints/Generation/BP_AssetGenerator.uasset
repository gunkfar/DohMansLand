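; BP_AssetGenerator procedurally populates the level with large, medium and small assets one tick after BeginPlay, if ShouldSpawn is set.
; The three spawn passes chain in size order, requesting random navmesh transforms over a wider radius for each smaller tier.
; SetSpawnableClass picks randomly among entries whose Frequency beats a random roll, then decrements that entry's remaining count, removing it when exhausted.
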(event Custom|SpawnLargeAssets
  ;[0.2 0.2 0.2] Spawns a set number of meshes with some variance into the game
  (for _index (range 0 (Variables|NumberOfAssets|GetMaxLargeAssets))
    (Game|SpawnActorfromClass (CallFunction|SetSpawnableClass (Variables|Default|GetLargeAssets)) (Utilities|RandomTransforminNavMesh 5e+03) "Undefined" self false 0))
  (CallFunction|SpawnMediumAssets))

(event Custom|SpawnMediumAssets
  ;[0.2 0.2 0.2] Spawns a set number of meshes with some variance into the game
  (for _index (range 0 (Variables|NumberOfAssets|GetMaxMediumAssets))
    (Game|SpawnActorfromClass (CallFunction|SetSpawnableClass (Variables|Default|GetMediumAssets)) (Utilities|RandomTransforminNavMesh 7.5e+03) "Undefined" self false 0))
  (CallFunction|SpawnSmallAssets))

(event Custom|SpawnSmallAssets
  ;[0.2 0.2 0.2] Spawns a set number of meshes with some variance into the game
  (for _index (range 0 (Variables|NumberOfAssets|GetMaxSmallAssets))
    (Game|SpawnActorfromClass (CallFunction|SetSpawnableClass (Variables|Default|GetSmallAssets)) (Utilities|RandomTransforminNavMesh 1e+04) "Undefined" self false 0)))

(event EventBeginPlay
  ;[0.2 0.2 0.2] Sorts meshes based on area of one side
  (Utilities|FlowControl|DelayUntilNextTick)
  (if (Variables|Default|GetbShouldSpawn)
    (CallFunction|SpawnLargeAssets)))

(fn ConstructionScript)

(fn SetSpawnableClass
  (params (AssetArray :type Array%20of%20F%20Asset%20Spawning%20Info%20Structures))
  ;[1 1 1] choose random mesh to spawn
  (LocalVariables|SetRandomFloat (Math|Random|RandomFloat))
  (for _array_element AssetArray
    (if (> (.Frequency (Utilities|Struct|BreakFAssetSpawningInfo _array_element)) (LocalVariables|GetRandomFloat))
      (Utilities|Array|Add (LocalVariables|GetPossibleClasses) _array_element)))
  (Utilities|FlowControl|Sequence
    (:then_0
      (LocalVariables|SetSpawningData (.OutItem (Utilities|Array|Random (LocalVariables|GetPossibleClasses)))))
    (:then_1
      (if (<= (- (.maxnumberspawned (LocalVariables|GetSpawningData)) 1) 0)
        (Utilities|Array|RemoveItem AssetArray (LocalVariables|GetSpawningData))
        (else
          (LocalVariables|SetReplacementIndex (Utilities|Array|FindItem AssetArray (LocalVariables|GetSpawningData)))
          (Utilities|Array|RemoveItem AssetArray (LocalVariables|GetSpawningData))
          (Utilities|Array|Insert AssetArray (Utilities|Struct|MakeFAssetSpawningInfo (.class (LocalVariables|GetSpawningData)) (- (.maxnumberspawned (LocalVariables|GetSpawningData)) 1) (.frequency (LocalVariables|GetSpawningData))) (LocalVariables|GetReplacementIndex)))))
    (:then_2
      (return (.class (LocalVariables|GetSpawningData))))))