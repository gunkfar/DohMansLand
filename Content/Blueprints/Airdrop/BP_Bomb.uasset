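; Timed bomb actor with a burning fuse that explodes, radially impulses physics-simulating components within ExplosionRadius, then destroys itself with a camera shake.
; Construction builds spline-mesh wick segments along the Fuze spline and sizes the range particles to that radius.
; On BeginPlay, FuseTimer drives the wick material's length and triggers the explosion when finished.
; A separate FuseMovement timeline, rate-scaled by FuseSpeed, moves the spark backwards along the spline.
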(event Custom|Explode
  (bind _mesh (Variables|Default|GetMesh))
  (bind _returnvalue (Transformation|GetWorldLocation _mesh))
  ;[0.2 0.2 0.2] Explode anything within the ExplosionRadius, and Impulse anything in the ImpulseRadius
  (Niagara|SpawnSystematLocation "/Game/Assets/FX/AirDrops/FX_BombExplosion.FX_BombExplosion" (Transformation|GetWorldLocation (Variables|Default|GetMesh)))
  (Utilities|FlowControl|Delay 0.25)
  (bind _outhits (Collision|MultiSphereTraceByChannel _returnvalue _returnvalue (Variables|Default|GetExplosionRadius) "TraceTypeQuery3" false 0 "None"))
  (for _array_element _outhits
    (if (Physics|IsSimulatingPhysics (.HitComponent (Collision|BreakHitResult _array_element)) "None")
      (Physics|AddRadialImpulse (.HitComponent (Collision|BreakHitResult _array_element)) (Transformation|GetWorldLocation (Variables|Default|GetExplosionEpicenter)) (Variables|Default|GetExplosionRadius) (Variables|Default|GetImpulseStrength) "RIF_Constant" true)))
  (Actor|DestroyActor))

(event Custom|MoveFuse
  (bind _fuze (Variables|Default|GetFuze))
  ;[1 1 1] Moves fuse across the spline using timeline
  (Components|Timeline|SetPlayRate (Variables|Default|GetFuseMovement) (/ 1.0 (Variables|Default|GetFuseSpeed)))
  (bind _fuse (Timeline|FuseMovement Play)
    (:Update
      (Transformation|SetWorldTransform (Variables|Default|GetSpark) (Math|Transform|MakeTransform (Spline|GetLocationatDistanceAlongSpline _fuze (Math|Float|Lerp (Spline|GetSplineLength (Variables|Default|GetFuze)) 0.0 _fuse) "World") (Spline|GetRotationatDistanceAlongSpline _fuze (Math|Float|Lerp (Spline|GetSplineLength (Variables|Default|GetFuze)) 0.0 _fuse) "World") "1.000000,1.000000,1.000000") false false))))

(event EventBeginPlay
  ;[0.2 0.2 0.2] Lessens the length of the wick over time
  (Utilities|FlowControl|Sequence
    (:then_0
      (bind _fusetimer (Timeline|FuseTimer Play)
        (:Update
          (Rendering|Material|SetScalarParameterValue (Variables|Default|GetWickMaterial) "WickLength" _fusetimer :!class /Script/Engine.MaterialInstanceDynamic))
        (:Finished
          (CallFunction|Explode)
          (Audio|PlaySound2D "/Game/Assets/SFX/misc_outside_noises/Powerup_capsule/Capsule_explosion/SFXQ_powerup_explosion.SFXQ_powerup_explosion" 1.0 1.0 0.0 0 0))))
    (:then_1
      (Utilities|FlowControl|Delay 5.0)
      (Audio|PlaySound2D "/Game/Assets/SFX/misc_outside_noises/Powerup_capsule/Powerup_Beeping/SFXQ_Fuse.SFXQ_Fuse" 1.0 1.0 0.0 0 0))
    (:then_2
      (Niagara|SpawnSystematLocation 0 "0, 0, 0"))
    (:then_3
      (CallFunction|MoveFuse))))

(event EventDestroyed
  ;[0.2 0.2 0.2] Explode anything within the ExplosionRadius, and Impulse anything in the ImpulseRadius
  (CameraShakes|StartCameraShake (Game|GetPlayerCameraManager 0) "/Game/Blueprints/MapItems/Bp_CameraShake.Bp_CameraShake_C" 2.0 "CameraLocal" "0, 0, 0"))

(fn ConstructionScript
  (bind _fuze (Variables|Default|GetFuze))
  (Utilities|FlowControl|Sequence
    (:then_0
      (for _index (range 0 (- (Spline|GetNumberOfSplinePoints (Variables|Default|GetFuze)) 2))
        (bind _returnvalue (AddComponent|AddSplineMeshComponent false (Math|Transform|MakeTransform "6.000000,1.000000,440.000000" "90.000000,0.000000, 0" "1.000000,1.000000,1.000000")))
        (SplineMesh|SetStartandEnd _returnvalue (.Location (Spline|GetLocationandTangentatSplinePoint _fuze _index "Local")) (.Tangent (Spline|GetLocationandTangentatSplinePoint _fuze _index "Local")) (.Location (Spline|GetLocationandTangentatSplinePoint _fuze (+ _index 1) "Local")) (.Tangent (Spline|GetLocationandTangentatSplinePoint _fuze (+ _index 1) "Local")) true :!class /Script/Engine.SplineMeshComponent)
        (Collision|SetCollisionEnabled _returnvalue "QueryAndPhysics")
        (bind _returnvalue_2 (Rendering|Material|CreateDynamicMaterialInstance _returnvalue 0 "/Game/Assets/Materials/Bombs/M_BombWick.M_BombWick" "None" :!class /Script/Engine.PrimitiveComponent))
        (Variables|Default|SetWickMaterial _returnvalue_2)))
    (:then_2
      (Effects|Components|ParticleSystem|SetFloatParameter (Variables|Default|GetRangeParticles) "user.PushRange" (Variables|Default|GetExplosionRadius)))))