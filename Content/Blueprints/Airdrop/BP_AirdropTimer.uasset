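; Airdrop countdown timer whose rotating dial triggers a BP_AirdropPlane spawn each time it completes a cycle.
; Game start begins a looping timer that steps the dial every sixtieth of the cooldown.
; Near zero yaw, it spawns the plane at a randomly rotated offset with sound, then a timeline rewinds the dial and restarts with a random cooldown.
; SetSpawnableClass picks a class from weighted SpawnablesMap, but is not called here.
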(event Custom|ResetCountdown
  ;[0.2 0.2 0.2] Rewinds timer after airdrop is dropped
  (bind _newrotation (Timeline|WindTimer PlayFromStart)
    (:Update
      (Transformation|SetRelativeRotation (Variables|Default|GetTimerDial) (Math|Rotator|MakeRotator 0.0 0.0 _newrotation) false false))
    (:Finished
      (Variables|Default|SetCooldown (select (Variables|Default|GetbInitialSpawn) (Variables|Default|GetCooldown) (Math|Random|RandomFloatinRange (Variables|Default|GetMinCooldown) (Variables|Default|GetMaxCooldown))))
      (CallFunction|StartTimer))))

(event Custom|TickTimer
  (bind _returnvalue (Math|Random|RandomFloatinRange -1.8e+02 1.8e+02))
  (bind _timerdial (Variables|Default|GetTimerDial))
  (bind _returnvalue_2 (Math|Vector|RotateVectorAroundAxis "8000.000000,10000.000000,2000.000000" _returnvalue "0, 0,1.000000"))
  ;[0.2 0.2 0.2] Ticks the timer depending on the cooldown
  (Transformation|AddRelativeRotation _timerdial (Math|Rotator|MakeRotator 0.0 0.0 -6.0) false false)
  (if (Math|Float|NearlyEqual(Float) (.yaw (Variables|/Script/Engine.SceneComponent|GetRelativeRotation _timerdial)) 0.0 2.0)
    (Game|SpawnActorfromClass "/Game/Blueprints/Airdrop/BP_AirdropPlane.BP_AirdropPlane_C" (Math|Transform|MakeTransform _returnvalue_2 (Math|Rotator|FindLookatRotation _returnvalue_2 (Math|Vector|MakeVector 0.0 0.0 5e+03)) "1.000000,1.000000,1.000000") "Undefined" 0 (Variables|Default|GetNav%20Data) 0)
    (Utilities|FlowControl|Sequence
      (:then_0
        (CallFunction|ResetCountdown)
        (Utilities|Time|ClearandInvalidateTimerbyHandle (Variables|Default|GetTimerHandle)))
      (:then_1
        (bind _returnvalue_3 (Actor|GetActorOfClass "/Game/Blueprints/Airdrop/BP_AirdropPlane.BP_AirdropPlane_C"))
        (Audio|PlaySoundatLocation "/Game/Assets/SFX/misc_outside_noises/Powerup_capsule/Dropping/SFXQ_powerup_dropping_sound.SFXQ_powerup_dropping_sound" (Transformation|GetActorLocation _returnvalue_3) "0, 0, 0" 1.0 1.0 0.0 0 0 0 0)))))

(event Custom|StartTimer
  ;[0.2 0.2 0.2] Timer only starts ticking when a player is spawned in
  (bind _returnvalue (Utilities|Time|SetTimerbyEvent (delegate Custom|TickTimer) (/ (Variables|Default|GetCooldown) 6e+01) true))
  (Variables|Default|SetTimerHandle _returnvalue)
  (Variables|Default|SetbInitialSpawn false))

(event EventBeginPlay
  ;[0.2 0.2 0.2] Timer only starts ticking when a player is spawned in
  (EventDispatchers|BindEventtoGameStart (CallFunction|GetDohMansLandGameMode) (delegate Custom|StartTimer)))

(fn ConstructionScript)

(fn SetSpawnableClass
  (bind _spawnablesmap (Variables|Default|GetSpawnablesMap))
  ;[0.2 0.2 0.2] Gets a class to spawn based on a probability set in SpawnablesMap, lower number = lower probability
  (LocalVariables|SetRandomFloat (Math|Random|RandomFloatinRange 0.0 1e+01))
  (bind _keys (Utilities|Map|Keys _spawnablesmap))
  (for _array_element _keys
    (if (> (.Value (Utilities|Map|Find _spawnablesmap _array_element)) (LocalVariables|GetRandomFloat))
      (LocalVariables|SetClassToSpawn _array_element)))
  (return (LocalVariables|GetClassToSpawn)))