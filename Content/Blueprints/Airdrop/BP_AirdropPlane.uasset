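; Airdrop plane that flies forward while spinning its propeller and drops powerups or bombs along the way.
; A looping timer, with an interval randomized once at BeginPlay, is set up to drive spawning at the plane's location while it is inside a fixed box.
; Spawning stops after three drops of any type.
; Each class is picked by comparing a random roll to SpawnablesMap thresholds, with the last match winning.
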(event Custom|SpawnAirdrops
  (bind _returnvalue (Transformation|GetActorLocation))
  ;[0.2 0.2 0.2] spawn airdrops
  (if (Math|Geometry|IsPointinBox (Math|Vector|MakeVector (.x _returnvalue) (.y _returnvalue) 0.0) "0, 0, 0" "5000.000000,10000.000000,10.000000")
    (if (== (Variables|Default|GetMaxPowerupsSpawned) 3)
      (Utilities|Time|ClearandInvalidateTimerbyHandle (Variables|Default|GetSpawnTimerHandle))
      (else
        (Math|Integer|IncrementInt (Variables|Default|GetMaxPowerupsSpawned)
          (:%20%20
            (Game|SpawnActorfromClass (CallFunction|SetSpawnablesClass) (Math|Transform|MakeTransform (Transformation|GetActorLocation) "0, 0, 0" "1.000000,1.000000,1.000000") "Undefined" 0 0)))))))

(event EventTick
  (params (DeltaSeconds :type Float%20%28single-precision%29))
  ;[0.2 0.2 0.2] move the plane across the screen
  (Transformation|AddActorLocalOffset (Math|Vector|MakeVector (* DeltaSeconds (Variables|Default|GetPlaneSpeed)) 0.0 0.0) true true)
  (Transformation|AddLocalRotation (Variables|Default|GetPropeller) "0, 0,20.000000" false false))

(event EventBeginPlay
  ;[0.2 0.2 0.2] set timer for spawning airdrops randomly
  (bind _returnvalue (Utilities|Time|SetTimerbyEvent (EventDispatchers|CreateEvent :!event Custom|SpawnAirdrops) (Math|Random|RandomFloatinRange 0.5 1.5) true))
  (Variables|Default|SetSpawnTimerHandle _returnvalue))

(fn ConstructionScript)

(fn SetSpawnablesClass
  (bind _spawnablesmap (Variables|Default|GetSpawnablesMap))
  ;[1 1 1] chooses to either spawn a powerup or bomb
  (LocalVariables|SetRandomFloat (Math|Random|RandomFloatinRange 0.0 1e+01))
  (bind _keys (Utilities|Map|Keys _spawnablesmap))
  (for _array_element _keys
    (if (> (.Value (Utilities|Map|Find _spawnablesmap _array_element)) (LocalVariables|GetRandomFloat))
      (LocalVariables|SetClassToSpawn _array_element)))
  (return (LocalVariables|GetClassToSpawn)))