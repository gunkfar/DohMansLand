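; Airdrop crate holding a random powerup that tanks can collect once its capsule is opened.
; Construction picks the powerup from an array, randomizes the roll and sets the billboard decal from the game mode's DecalMap.
; Projectiles call OpenCapsule, which removes capsule and cap with effects and enables pickup through box overlap.
; A timer fires shortly before lifespan expiry to shrink the capsule with a timeline.
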(event OnComponentBeginOverlap(Box)
  (params (OverlappedComponent :type Primitive%20Component%20Object%20Reference) (OtherActor :type Actor%20Object%20Reference) (OtherComp :type Primitive%20Component%20Object%20Reference) (OtherBodyIndex :type Integer) (bFromSweep :type Boolean) (SweepResult :type Hit%20Result%20Structure%20%28by%20ref%29))
  ;[0.2 0.2 0.2] Adds the powerup to the tank when it is run into
  (if (Variables|Default|GetbCanBeCollected)
    (bind _asbp_base_tank (Utilities|Casting|CastToBP_BaseTank OtherActor))
    (Default|AddPowerup _asbp_base_tank (Variables|Powerups|GetPowerup))
    (Actor|DestroyActor)))

(event Custom|ShrinkOnAutoDestroy
  (bind _scale (Timeline|ShrinkTimeline Play)
    (:Update
      (Transformation|SetWorldScale3D (Variables|Default|GetCapsule) _scale))))

(event Custom|OpenCapsule
  ;[0.2 0.2 0.2] Called from BP_BaseProjectile, opens the capsule and makes the powerup collectable
  (if (not (Variables|Default|GetbHasBeenOpened))
    (Variables|Default|SetbCanBeCollected true)
    (Audio|PlaySoundatLocation "/Game/Assets/SFX/misc_outside_noises/Powerup_capsule/Capsule_pop/SFXQ_pop.SFXQ_pop" (Transformation|GetWorldLocation (Variables|Default|GetCapsule)) "0, 0, 0" 1.0 1.0 0.0 0 0 0 0)
    (Components|DestroyComponent (Variables|Default|GetCapsule))
    (Niagara|SpawnSystematLocation "/Game/Assets/FX/AirDrops/FX_OpenCapsule.FX_OpenCapsule" (Transformation|GetActorLocation) "0, 0, 0" "10.000000,10.000000,10.000000")
    (Variables|Default|SetbHasBeenOpened true)))

(event EventBeginPlay
  (Utilities|Time|SetTimerbyEvent (delegate Custom|ShrinkOnAutoDestroy) (- (Variables|Actor|GetInitialLifeSpan) (Math|Random|RandomFloatinRange 2.0 3.0))))

(fn ConstructionScript
  ;[0.2 0.2 0.2] Initialization for deciding what powerup will spawn
  (Variables|Default|SetPowerupIndex (Math|Random|RandomIntegerinRange 0 (- (Utilities|Array|Length (Variables|Powerups|GetPowerupArray)) 1)))
  (Transformation|SetActorRotation (Math|Rotator|MakeRotator (Math|Random|RandomFloatinRange -6e+01 -1.8e+02) 0.0 0.0) true)
  ;[0.2 0.2 0.2] Sets what powerup will spawn + sets the decal to display in the capsule
  (Variables|Powerups|SetPowerup (Utilities|Array|Get(acopy) (Variables|Powerups|GetPowerupArray) (Variables|Default|GetPowerupIndex)))
  (Rendering|Material|SetMaterial (Variables|Default|GetMaterialBillboard) 0 (.Value (Utilities|Map|Find (Variables|/Game/Blueprints/Player/BP_DohMansLand_GameMode.BP_DohMansLand_GameMode_C|GetDecal%20Map (CallFunction|GetDohMansLandGameMode)) (Variables|Powerups|GetPowerup)))))